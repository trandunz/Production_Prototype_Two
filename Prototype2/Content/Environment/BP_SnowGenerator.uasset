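; Geometry Script generator that builds a snow mesh over upward-facing surfaces of chosen actors.
; GenerateMeshCache merges their root-component meshes in world space and builds a BVH.
; On rebuild, a grid of downward rays appends spheres at hits passing a SnowCoverage normal test, then converts them to actor space.
; Optional remeshing fuses them with morphology and smoothing, then rebuilds UVs, tangents and normals; a random-scatter variant is left unconnected.
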(event `GenerateMeshCache`
  (`|ExecutionSequence`
    (:`then_0`
      ;[0 0 0] Allows Multiple Meshes to have Snow Added to them
      (bind _returnvalue (`self.AllocateComputeMesh`))
      (set `self.RaycastMeshActors` _returnvalue)
      (for _array_element (`self.MeshesToAddSnowTo`)
        (bind _returnvalue_2 (`self.AllocateComputeMesh`))
        (bind (_localtoworld _returnvalue_3) (`GeometryScriptLibrary_SceneUtilityFunctions.CopyMeshFromComponent` (`Actor.RootComponent` _array_element) _returnvalue_2 (struct) true null)
          (:`Failure`
            _)
          (:`Success`
            (`GeometryScriptLibrary_MeshBasicEditFunctions.AppendMesh` (`self.RaycastMeshActors`) _returnvalue_3 (struct) false (struct :`CombineMode` "EnableAllMatching") null)))
        (`self.ReleaseComputeMesh` _returnvalue_2)))
    (:`then_1`
      (bind _outputbvh (`GeometryScriptLibrary_MeshSpatial.BuildBVHForMesh` (`self.RaycastMeshActors`) null))
      (set `self.Output BVH` _outputbvh))))

(event `self.OnRebuildGeneratedMesh`
  (params (TargetMesh :type "DynamicMesh Object Reference"))
  (bind _returnvalue (`GeometryScriptLibrary_MeshQueryFunctions.GetMeshBoundingBox` (`self.RaycastMeshActors`)))
  (set `self.Target Mesh` TargetMesh)
  (if (`self.Generate Snow`)
    (`|ExecutionSequence`
      (:`then_0`
        ;[0 0 0] X Axis Spacing
        (for _index (range (+ (`KismetMathLibrary.Round` (/ (- (.x (`.Max` (break `Box` _returnvalue))) (.x (break `Box` _returnvalue))) (`self.GridSpacing`))) 1))
          ;[0 0 0] Y Axis Spacing
          (for _index_2 (range (+ (`KismetMathLibrary.Round` (/ (- (.y (`.Max` (break `Box` _returnvalue))) (.y (break `Box` _returnvalue))) (`self.GridSpacing`))) 1))
            (bind _hitresult (`GeometryScriptLibrary_MeshSpatial.FindNearestRayIntersectionWithMesh` (`self.RaycastMeshActors`) (`self.Output BVH`) (`KismetMathLibrary.MakeVector` (+ (.x (break `Box` _returnvalue)) (* _index (`self.GridSpacing`))) (+ (.y (break `Box` _returnvalue)) (* _index_2 (`self.GridSpacing`))) (+ (- (.z (`.Max` (break `Box` _returnvalue))) (.z (break `Box` _returnvalue))) 1000.0)) (0.0 0.0 -1.0) (struct) null)
              (:`Found`
                (if (>= (.z (`.ReturnValue` (`GeometryScriptLibrary_MeshQueryFunctions.GetTriangleFaceNormal` (`self.RaycastMeshActors`) (`.HitTriangleID` (break `GeometryScriptRayHitResult` _hitresult))))) (`KismetMathLibrary.Abs` (- (`self.SnowCoverage`) 1.5)))
                  (`GeometryScriptLibrary_MeshPrimitiveFunctions.AppendSphereBox` (`self.Target Mesh`) (struct) (`KismetMathLibrary.MakeTransform` (`.HitPosition` (break `GeometryScriptRayHitResult` _hitresult))) (`self.SphereRadius`) 6 6 6 "Center" null)))))))
      (:`then_1`
        ;[0 0 0] Change Transforms of Appended Spheres from Local to World
        (`GeometryScriptLibrary_MeshTransformFunctions.TransformMesh` (`self.Target Mesh`) (`KismetMathLibrary.InvertTransform` (`self.GetTransform`)) true null))
      (:`then_2`
        ;[0 0 0] Remesh the Spheres to look more like Snow
        (if (`self.Remesh`)
          (bind _returnvalue_2 (`GeometryScriptLibrary_MeshVoxelFunctions.ApplyMeshMorphology` (`self.Target Mesh`) (make `GeometryScriptMorphologyOptions` (make `GeometryScript3DGridParameters` "GridResolution") false (make `GeometryScript3DGridParameters` "GridResolution") "Dilate" (`self.SnowThickness`)) null))
          (bind _returnvalue_3 (`GeometryScriptLibrary_MeshDeformFunctions.ApplyIterativeSmoothingToMesh` _returnvalue_2 (struct) (make `GeometryScriptIterativeMeshSmoothingOptions` (`self.SmoothIterations`)) null))
          (bind (_returnvalue_min _returnvalue_max) (break `Box` (`GeometryScriptLibrary_MeshQueryFunctions.GetMeshBoundingBox` _returnvalue_3)))
          (bind _returnvalue_4 (`GeometryScriptLibrary_MeshUVFunctions.SetMeshUVsFromBoxProjection` _returnvalue_3 0 (`KismetMathLibrary.MakeTransform` (0.0 0.0 0.0) (struct) (- _returnvalue_max _returnvalue_min)) (struct) 2 null))
          (bind _returnvalue_5 (`GeometryScriptLibrary_MeshNormalsFunctions.ComputeTangents` _returnvalue_4 (struct) null))
          (`GeometryScriptLibrary_MeshNormalsFunctions.ComputeSplitNormals` _returnvalue_5 (make `GeometryScriptSplitNormalsOptions` true 80.0) (struct) null))))))

(fn `UserConstructionScript`)