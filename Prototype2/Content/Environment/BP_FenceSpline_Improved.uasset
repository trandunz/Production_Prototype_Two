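; Construction-script fence builder that lays deformed mesh segments along an editable spline, with an optional closed loop.
; It derives the segment count from spline length, then evens out segment length to fit.
; Each collidable spline mesh randomly gets one of two variants and uses tangents clamped to segment length.
; The last-mesh override is noted as broken; its component array is cleared but never filled.
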(fn `Randomise`
  (bind _mesh_component (`self.Mesh Component`))
  (set `self.SelectVariant` (`KismetMathLibrary.RandomIntegerInRange` 0 1))
  (for _ (range (+ (`self.indexSize`) 1))
    (switch `int` (`self.SelectVariant`)
      (:`0`
        (`StaticMeshComponent.SetStaticMesh` _mesh_component (`self.Mesh Var01`)))
      (:`1`
        (`StaticMeshComponent.SetStaticMesh` _mesh_component (`self.Mesh Var02`))))))

(fn `UserConstructionScript`
  (bind _spline_components (`self.Spline Components`))
  (bind _spline (`self.Spline`))
  (bind _mesh_component (`self.Mesh Component`))
  (`KismetArrayLibrary.Array_Clear` (`self.Spline Components`))
  (if (`self.Close Loop?`)
    (`SplineComponent.SetClosedLoop` (`self.Spline`) true true))
  (bind _output_get (set `self.indexSize` (`KismetMathLibrary.FTrunc` (/ (`SplineComponent.GetSplineLength` (`self.Spline`)) (`self.length`)))))
  (set `self.newLength` (/ (`SplineComponent.GetSplineLength` (`self.Spline`)) _output_get))
  (for _index (range (+ _output_get 1))
    (bind _returnvalue (`AddComponent|NODE_AddSplineMeshComponent-0`))
    (bind _output_get_2 (set `self.Mesh Component` _returnvalue))
    (`SplineMeshComponent.SetForwardAxis` _output_get_2 "X" true)
    (`self.Randomise`) ; Can change and randomise static meshes
    (`PrimitiveComponent.SetCollisionEnabled` _mesh_component "QueryAndPhysics")
    (bind _returnvalue_2 (* _index (`self.newLength`)))
    (bind _returnvalue_3 (* (`KismetMathLibrary.Conv_IntToDouble` (+ _index 1)) (`self.newLength`)))
    (`SplineMeshComponent.SetStartAndEnd` _mesh_component (`SplineComponent.GetLocationAtDistanceAlongSpline` _spline _returnvalue_2 "Local") (`KismetMathLibrary.ClampVectorSize` (`SplineComponent.GetTangentAtDistanceAlongSpline` _spline _returnvalue_2 "Local") 0.0 (`self.newLength`)) (`SplineComponent.GetLocationAtDistanceAlongSpline` _spline _returnvalue_3 "Local") (`KismetMathLibrary.ClampVectorSize` (`SplineComponent.GetTangentAtDistanceAlongSpline` _spline _returnvalue_3 "Local") 0.0 (`self.newLength`)) true))
  ;[1 1 1] Set Start and End Meshes? Not Working
  (`StaticMeshComponent.SetStaticMesh` (`|GetArrayItem` _spline_components (- (`KismetArrayLibrary.Array_Length` _spline_components) 1)) (`self.New Mesh`)) ; Meant to be able to change the last mesh but doesn't work
)