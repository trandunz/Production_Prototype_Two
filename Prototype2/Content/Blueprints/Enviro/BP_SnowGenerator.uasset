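; Geometry Script generator actor that builds a procedural snow mesh over the actors listed in MeshesToAddSnowTo.
; On rebuild, it merges their root-component meshes in world space into a compute mesh and builds a BVH.
; Seeded random downward rays across the bounds place small spheres at hit points.
; The result is transformed into actor-local space, with optional mesh morphology to remesh the spheres.
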(event `self.OnRebuildGeneratedMesh`
  (params (TargetMesh :type "DynamicMesh Object Reference"))
  (bind _stream (`self.Stream`))
  (set `self.Target Mesh` TargetMesh)
  (`|ExecutionSequence`
    (:`then_0`
      (bind _returnvalue (`self.AllocateComputeMesh`))
      (set `self.RaycastMeshActors` _returnvalue)
      (for _array_element (`self.MeshesToAddSnowTo`)
        (bind _returnvalue_2 (`self.AllocateComputeMesh`))
        (bind (_localtoworld _returnvalue_3) (`GeometryScriptLibrary_SceneUtilityFunctions.CopyMeshFromComponent` (`Actor.RootComponent` _array_element) _returnvalue_2 (struct) true null)
          (:`Failure`
            _)
          (:`Success`
            (`GeometryScriptLibrary_MeshBasicEditFunctions.AppendMesh` (`self.RaycastMeshActors`) _returnvalue_3 (struct) false (struct :`CombineMode` "EnableAllMatching") null)))
        (`self.ReleaseComputeMesh` _returnvalue_2)))
    (:`then_1`
      (bind (_outputbvh _returnvalue_4) (`GeometryScriptLibrary_MeshSpatial.BuildBVHForMesh` (`self.RaycastMeshActors`) null))
      (set `self.Output BVH` _outputbvh)
      (for _ (range (+ (`self.NumberOfSpheres`) 1))
        (bind _returnvalue_5 (`GeometryScriptLibrary_MeshQueryFunctions.GetMeshBoundingBox` _returnvalue_4))
        (bind _hitresult (`GeometryScriptLibrary_MeshSpatial.FindNearestRayIntersectionWithMesh` (`self.RaycastMeshActors`) (`self.Output BVH`) (`KismetMathLibrary.MakeVector` (`KismetMathLibrary.RandomFloatInRangeFromStream` (.x (break `Box` _returnvalue_5)) (.x (`.Max` (break `Box` _returnvalue_5))) _stream) (`KismetMathLibrary.RandomFloatInRangeFromStream` (.y (break `Box` _returnvalue_5)) (.y (`.Max` (break `Box` _returnvalue_5))) _stream) (+ (- (.z (`.Max` (break `Box` _returnvalue_5))) (.z (break `Box` _returnvalue_5))) 1000.0)) (0.0 0.0 -1.0) (struct) null)
          (:`Found`
            (`GeometryScriptLibrary_MeshPrimitiveFunctions.AppendSphereBox` (`self.Target Mesh`) (struct) (`KismetMathLibrary.MakeTransform` (`.HitPosition` (break `GeometryScriptRayHitResult` _hitresult))) 6.0 6 6 6 "Center" null)))))
    (:`then_2`
      (`GeometryScriptLibrary_MeshTransformFunctions.TransformMesh` (`self.Target Mesh`) (`KismetMathLibrary.InvertTransform` (`self.GetTransform`)) true null))
    (:`then_3`
      (if (`self.Remesh`)
        (`GeometryScriptLibrary_MeshVoxelFunctions.ApplyMeshMorphology` (`self.Target Mesh`) (struct) null)))))

(fn `UserConstructionScript`)