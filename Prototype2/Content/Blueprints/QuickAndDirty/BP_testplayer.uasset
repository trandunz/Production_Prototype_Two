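; BP_testplayer is a quick test player Blueprint that supplies visual feedback for weapon attacks.
; TriggerAttackVFX draws a debug circle at the attack position, sized by radius and thickened by charge.
; StretchWeapon and SquashWeapon use timelines to scale the weapon mesh for squash-and-stretch.
; When the squash finishes, a short delay precedes re-socketing the weapon to its held socket.
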(event `Key|Q`
  (params (Key :type "Key Structure")))

(event `self.TriggerAttackVFX`
  (params (Position :type "Vector Structure") (Radius :type "Float (single-precision)") (Charge :type "Float (single-precision)"))
  (`KismetSystemLibrary.DrawDebugCircle` Position Radius 100 (struct :`R` 1.0 :`B` 0.87436 :`A` 1.0) 1.0 Charge (0.0 1.0 0.0) (1.0 0.0 0.0)))

(event `self.StretchWeapon`
  (bind (_direction _newtrack_0) (`Timeline|Stretch_Timeline` :!via `PlayFromStart`)
    (:`Update`
      (`SceneComponent.SetWorldScale3D` (`Weapon.Mesh` (`self.Weapon`)) (`KismetMathLibrary.MakeVector_NetQuantize` 3.0 3.0 _newtrack_0)))))

(event `self.SquashWeapon`
  (bind (_direction _x _z _y) (`Timeline|Squash_Timeline` :!via `PlayFromStart`)
    (:`Update`
      (`SceneComponent.SetWorldScale3D` (`Weapon.Mesh` (`self.Weapon`)) (`KismetMathLibrary.MakeVector_NetQuantize` _y _x _z)))
    (:`Finished`
      (`KismetSystemLibrary.Delay` 0.2)
      (`self.SocketWeapon` "WeaponHeldSocket"))))

(fn `UserConstructionScript`)